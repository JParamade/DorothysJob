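; Player Blueprint for Dorothy that sets up the audio listener and aim assist for ranged weapons.
; CalculateAimAssist turns the muzzle toward the closest room enemy inside a weapon-specific angle, using a line trace to reject targets behind obstacles.
; Helpers identify the equipped WasheeFlashee or Dirtminator and fetch room enemies from the level manager.
; Without a current room it assumes the hub, targeting a once-cached BP_MrsClean (Skelly) with a narrower angle.
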(event `self.ReceiveBeginPlay`
  ;[1 0.4727 0 0.5] begin play
  (`|ExecutionSequence`
    (:`then_0`
      (`PlayerController.SetAudioListenerOverride` (`GameplayStatics.GetPlayerController` 0) (`self.m_pCollisionComponent`) (0.0 0.0 0.0) (struct :`Yaw` -45.0))
      (`KismetSystemLibrary.Delay` 1.0)
      (`AnimInstance.Montage_SetPlayRate` (`SkeletalMeshComponent.GetAnimInstance` (`self.m_pMeshComponent`)) "/Game/Characters/Player/Animations/Mopressor/AM_CHR_Dorothy_Mopressor.AM_CHR_Dorothy_Mopressor" 10.0)
      (`KismetSystemLibrary.Delay` 2.0) ; tiempo de cortesía
      (`self.getEnemiesInRoom`) ; this will go out of the do once\nand record the skelly reference\nforever if we are in the hub room
    )))

(event `self.CalculateAimAssist`
  (bind (_returnvalue_roll _returnvalue_pitch _returnvalue_yaw) (`KismetMathLibrary.BreakRotator` (`KismetMathLibrary.Conv_VectorToRotator` (`SceneComponent.GetForwardVector` (`self.m_pMeshComponent`)))))
  (bind (_returnvalue_roll_2 _returnvalue_pitch_2 _returnvalue_yaw_2) (`KismetMathLibrary.BreakRotator` (`KismetMathLibrary.Conv_VectorToRotator` (- (`self.K2_GetActorLocation` (`self.skellyReference`)) (`self.K2_GetActorLocation`)))))
  ;[0 0.5094 1 0.5] aim assist stoof
  (`self.recordCurrentWeapon`)
  (`SceneComponent.K2_SetWorldRotation` (`self.GetMuzzle`) (`KismetMathLibrary.MakeRotator` 0.0 0.0 _returnvalue_yaw) false false) ; reset the rotation to the same as dorothy
  (bind _returnvalue (`self.getEnemiesInRoom`)
    (:`then`
      (bind _output_get (set `self.enemiesInRoom` _returnvalue))
      (set `self.correctedRotation` 0.0)
      (set `self.closestEnemyDistance` 3000.0) ; return it to 3000  para que el primero\nsiempre sea mas close que el
      (for _array_element _output_get
        (`/Engine/EditorBlueprintResources/StandardMacros.IsValid` _array_element
          (:`Is Valid`
            (bind _asbase_enemy (cast `BaseEnemy` _array_element))
            (if (< (`self.smallestAngleBetweenTwoVectors` _asbase_enemy) (select `byte` (`self.currentWeaponByte`) :`0` (`self.aimAssistOffset_WF`) :`1` (`self.aimAssistOffset_DMT`)))
              (bind _returnvalue_2 (`KismetMathLibrary.Vector_Distance` (`self.K2_GetActorLocation` _asbase_enemy) (`self.K2_GetActorLocation`)))
              (if (< _returnvalue_2 (`self.closestEnemyDistance`))
                (set `self.closestEnemyDistance` _returnvalue_2) ; i am now the closest distance
                (bind (_outhit _returnvalue_3) (`KismetSystemLibrary.LineTraceSingleByProfile` (`self.K2_GetActorLocation`) (`self.K2_GetActorLocation` _asbase_enemy) "BlockAllDynamic" false _returnvalue "None" true (struct :`R` 0.12264 :`B` 1.0 :`A` 1.0) (struct :`G` 0.670886 :`B` 1.0 :`A` 1.0))) ; cast a line from dorothy to momptur, only blocked by tables\nand furniture
                (if (not _returnvalue_3)
                  (bind (_returnvalue_roll_3 _returnvalue_pitch_3 _returnvalue_yaw_3) (`KismetMathLibrary.BreakRotator` (`KismetMathLibrary.Conv_VectorToRotator` (- (`self.K2_GetActorLocation` _asbase_enemy) (`self.K2_GetActorLocation`)))))
                  (set `self.correctedRotation` _returnvalue_yaw_3)
                  (goto _label :!via `Open`)))))))
      (`|ExecutionSequence`
        (:`then_0`
          (`/Engine/EditorBlueprintResources/StandardMacros.Gate` true :!label _label ; did i change the rotation?\nif i did, set the muzzle world \nrotation to the new corrected angle
            (:`Exit`
              (`SceneComponent.K2_SetWorldRotation` (`self.GetMuzzle`) (`KismetMathLibrary.MakeRotator` 0.0 0.0 (`self.correctedRotation`)) false false))))
        (:`then_1`
          (goto _label :!via `Close`))))
    (:`iAmInHub`
      ;;[0.1457 0 1 0.5] skelly aim assist
      (`|ExecutionSequence`
        (:`then_0`
          (if (< (`self.smallestAngleBetweenTwoVectors` (`self.skellyReference`)) (- (select `byte` (`self.currentWeaponByte`) :`0` (`self.aimAssistOffset_WF`) :`1` (`self.aimAssistOffset_DMT`)) 14.0))
            (goto _label_2 :!via `Open`)))
        (:`then_1`
          (`|ExecutionSequence`
            (:`then_0`
              (`/Engine/EditorBlueprintResources/StandardMacros.Gate` true :!label _label_2 ; must  i change the rotation?\nif i must, set the muzzle world \nrotation to the new corrected angle
                (:`Exit`
                  (`SceneComponent.K2_SetWorldRotation` (`self.GetMuzzle`) (`KismetMathLibrary.MakeRotator` 0.0 0.0 _returnvalue_yaw_2) false false))))
            (:`then_1`
              (goto _label_2 :!via `Close`))))))))

(fn `UserConstructionScript`)