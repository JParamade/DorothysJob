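; BP_OZ_OozerBaby is the baby Oozer enemy Blueprint, and its graph handles audio feedback for death and status effects.
; On BeginPlay it binds to the enemy-eliminate and state-changed events.
; Elimination plays the shared Oozer death voice at the mesh location, setting an "isBabe" parameter on the sound instance to mark the baby variant.
; Applied Slow, Exposure and Stun statuses each play their matching effect sound at the same location.
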(event `self.ReceiveBeginPlay`
  (add `self.OnEnemyEliminate` (delegate `OnEnemyEliminate_Event`))
  (add `self.OnStateChanged` (delegate `CustomEvent`)))

(event `CustomEvent` :!signature `self.OnStateChanged`
  (params (Status :type "BaseStatus Object Reference") (bApplied :type Boolean))
  (bind _returnvalue (`SceneComponent.K2_GetComponentLocation` (`self.m_pMeshComponent`)))
  (if bApplied
    (switch `EStatus` (`BaseStatus.GetStatusType` Status)
      (:`SLOW`
        (`FMODBlueprintStatics.PlayEventAtLocation` "/Game/FMOD/Events/SoundFX/Characters/Enemies/General/SFX_ENE_slowEffect.SFX_ENE_slowEffect" (`KismetMathLibrary.MakeTransform` _returnvalue)))
      (:`EXPOSURE`
        (`FMODBlueprintStatics.PlayEventAtLocation` "/Game/FMOD/Events/SoundFX/Characters/Enemies/General/SFX_ENE_exposureEffect.SFX_ENE_exposureEffect" (`KismetMathLibrary.MakeTransform` _returnvalue)))
      (:`STUN`
        (`FMODBlueprintStatics.PlayEventAtLocation` "/Game/FMOD/Events/SoundFX/Characters/Enemies/General/SFX_ENE_stunEffect.SFX_ENE_stunEffect" (`KismetMathLibrary.MakeTransform` _returnvalue))))))

(event `OnEnemyEliminate_Event` :!signature `self.OnEnemyEliminate`
  (params (_pPawn :type "BaseEnemy Object Reference"))
  ; death
  (bind _returnvalue (`FMODBlueprintStatics.PlayEventAtLocation` "/Game/FMOD/Events/SoundFX/Characters/Enemies/Oozers/SFX_ENE_oozer_deathVoice.SFX_ENE_oozer_deathVoice" (`KismetMathLibrary.MakeTransform` (`SceneComponent.K2_GetComponentLocation` (`self.m_pMeshComponent`)))))
  (`FMODBlueprintStatics.EventInstanceSetParameter` _returnvalue "isBabe" 1.0))

(fn `UserConstructionScript`)