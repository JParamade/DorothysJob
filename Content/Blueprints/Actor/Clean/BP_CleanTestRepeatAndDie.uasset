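; Test actor that repeatedly cleans or dirties an ooze area through its Drawing object, then destroys itself.
; BeginPlay and the Drawing's OnFloorFound event both feed an initial delay, which starts a timed loop and a fixed three-second self-destruct.
; Each loop pass calls Clean or Dirt, chosen by the Clean flag, stamping ooze textures at the configured size, with color and tier for dirt.
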(event `self.ReceiveBeginPlay`
  (bind _drawing (`self.Drawing`))
  (bind _drawing_2 (`self.Drawing`))
  (add `Drawing.OnFloorFound` (`self.Drawing`) (delegate `OnFloorFound_Event`))
  (`KismetSystemLibrary.Delay` (`self.InicialDuration`) :!label _label)
  (`|ExecutionSequence`
    (:`then_0`
      (`KismetSystemLibrary.Delay` (`self.Duration`) :!label _label_2)
      (if (`self.Clean`)
        (`/Engine/EditorBlueprintResources/StandardMacros.IsValid` _drawing
          (:`Is Valid`
            (`Drawing.Clean` _drawing "/Game/Graphics/Sprites/Cleaning/T_OozeReversed.T_OozeReversed" (`self.Size`) 0.0 (0.5 0.5))
            (goto _label_2)))
        (else
          (`/Engine/EditorBlueprintResources/StandardMacros.IsValid` _drawing_2
            (:`Is Valid`
              (`Drawing.Dirt` _drawing_2 "/Game/Graphics/Sprites/Cleaning/T_Ooze.T_Ooze" "/Game/Graphics/Sprites/Cleaning/T_OozeReversed.T_OozeReversed" (`self.Size`) 0.0 (0.5 0.5) (`self.Color Draw`) (`self.Tier Draw`))
              (goto _label_2))))))
    (:`then_1`
      (`KismetSystemLibrary.Delay` 3.0)
      (`self.K2_DestroyActor`))))

(event `OnFloorFound_Event`
  (goto _label))

(fn `UserConstructionScript`)