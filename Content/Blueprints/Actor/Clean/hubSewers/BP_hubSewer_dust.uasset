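; Hub sewer spawner that keeps a BP_DustPoop present at one fixed world position once the game instance's current level is 2 or higher.
; After a short startup delay for the floors to be created, it spawns the first one and binds to its destruction.
; Each destruction waits SewerCooldown, plays a formation sound and respawns it, keeping the first spawn silent during loading.
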(event `self.ReceiveBeginPlay`
  ;[1 0.2439 0 0.5] begin play
  (bind _asbase_game_instance (cast `BaseGameInstance` (`GameplayStatics.GetGameInstance`)))
  (if (>= (`BaseGameInstance.m_iCurrentLevel` _asbase_game_instance) 2)
    (`KismetSystemLibrary.Delay` 4.0) ; espera un tiempo de cortesia a\nque se creen los suelos
    (`self.createDustPoop`)))

(event `createDustPoop`
  ;[0.9957 1 0 0.5] create an infinite amount of dust poops
  (bind _returnvalue (`|SpawnActorFromClass` "/Game/Blueprints/Actor/Dust/BP_DustPoop.BP_DustPoop_C" (`KismetMathLibrary.MakeTransform` (-160.0 -850.0 113.0)) "Undefined" "MultiplyWithRoot" null null)) ; crea una dust speck en estas coordenadas exactas
  (bind _output_get (set `self.dustPoop_reference` _returnvalue))
  (add `self.OnDestroyed` _output_get (delegate `myDustPoopWasDestroyed`)))

(event `myDustPoopWasDestroyed` :!signature `self.OnDestroyed`
  (params (DestroyedActor :type "Actor Object Reference"))
  ;[0.9957 1 0 0.5] create an infinite amount of dust poops
  (`KismetSystemLibrary.Delay` (`self.sewerCooldown`)) ; my dust speck got rekt. espera un poco\nde tiempo y luego crea otra
  (`FMODBlueprintStatics.PlayEvent2D` "/Game/FMOD/Events/SoundFX/Characters/Enemies/DustBunnies/SFX_ENE_dustBunny_dustSpeckFormation.SFX_ENE_dustBunny_dustSpeckFormation") ; lo pongo aqui para que no suene en el primer dust\npoop durante la pantalla de carga
  (`self.createDustPoop`))

(fn `UserConstructionScript`)