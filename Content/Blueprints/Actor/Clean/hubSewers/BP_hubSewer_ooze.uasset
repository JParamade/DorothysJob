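; Hub sewer ooze actor that repeatedly paints growing ooze dirt onto the floor through its Drawing component.
; A delayed loop, entered from BeginPlay and again on OnFloorFound, stamps the ooze texture at a random rotation, passing a reversed texture for cleaning.
; Each stamp steps through five sizes up to MaxSize, then the index resets and the sewer rests for a cooldown before repeating.
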(event `self.ReceiveBeginPlay`
  (bind _drawing (`self.Drawing`))
  (add `Drawing.OnFloorFound` (`self.Drawing`) (delegate `OnFloorFound_Event`))
  (`KismetSystemLibrary.Delay` 0.2 :!label _label)
  (`/Engine/EditorBlueprintResources/StandardMacros.IsValid` _drawing :!label _label_2
    (:`Is Valid`
      (if (> (`self.sizeIndex`) 4)
        (set `self.sizeIndex` 0) ; if i was bigger than 4, reset\nme back to 0 and then let me\nrest for a bit
        (`KismetSystemLibrary.Delay` (`self.sewerCooldown`)))
      (`Drawing.Dirt` _drawing "/Game/Graphics/Sprites/Cleaning/T_Ooze.T_Ooze" "/Game/Graphics/Sprites/Cleaning/T_OozeReversed.T_OozeReversed" (`self.getSizeBasedOnIndex`) (`KismetMathLibrary.RandomFloatInRange` 0.0 360.0) (0.5 0.5) (`self.Color Draw`) (`self.Tier Draw`))
      (`/Engine/EditorBlueprintResources/StandardMacros.IncrementInt` (`self.sizeIndex`)
        (:`  `
          (`KismetSystemLibrary.Delay` (`self.dirtLoopDuration`))
          (goto _label_2))))))

(event `OnFloorFound_Event`
  (goto _label))

(fn `UserConstructionScript`)