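; BP_HUBDoor is the HUB door actor, exposing open and close animation events with sound effects.
; Two timelines, slowed at BeginPlay, drive the motion: one spins the wheel mesh on pitch, the other swings the door mesh on yaw.
; Opening starts the wheel first and the door after a short delay.
; Closing reverses both timelines, door first and wheel slightly later.
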(event `self.ReceiveBeginPlay`
  ;[1 0.115 0 0.5] begin play
  ;;[1 0.115 0 0.5] timelines speed
  (`TimelineComponent.SetPlayRate` (`self.Cronograma`) 0.65)
  (`TimelineComponent.SetPlayRate` (`self.Cronograma_0`) 0.6))

(event `openDoorAnimation`
  (`FMODBlueprintStatics.PlayEvent2D` "/Game/FMOD/Events/SoundFX/NonDiegetic/Hub/SFX_HUB_exitDoor_open.SFX_HUB_exitDoor_open")
  (`|ExecutionSequence`
    (:`then_0`
      (`KismetSystemLibrary.Delay` 0.55)
      ;[0.06448 0 1 0.5] door opening
      (bind (_direction _delta) (`Timeline|Cronograma` :!via `PlayFromStart` :!label _label)
        (:`Update`
          (`SceneComponent.K2_SetRelativeRotation` (`self.doorieMesh`) (`KismetMathLibrary.MakeRotator` 0.0 0.0 (`KismetMathLibrary.Lerp` 0.0 20.0 _delta)) false false))))
    (:`then_1`
      ;[0 0.8322 1 0.5] wheel turning
      (bind (_direction_2 _delta_2) (`Timeline|Cronograma_0` :!via `PlayFromStart` :!label _label_2)
        (:`Update`
          (`SceneComponent.K2_SetRelativeRotation` (`self.wheelieMesh`) (`KismetMathLibrary.MakeRotator` 0.0 (`KismetMathLibrary.Lerp` 0.0 350.0 _delta_2)) false false))))))

(event `closeDoorAnimation`
  (`FMODBlueprintStatics.PlayEvent2D` "/Game/FMOD/Events/SoundFX/Miscellaneous/Hub/SFX_HUB_door_close.SFX_HUB_door_close")
  (`|ExecutionSequence`
    (:`then_0`
      (goto _label :!via `ReverseFromEnd`))
    (:`then_1`
      (`KismetSystemLibrary.Delay` 0.4)
      (goto _label_2 :!via `ReverseFromEnd`))))

(fn `UserConstructionScript`)