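; BP_CleaningCupboard is an interactable cleaning cupboard actor that shows its current cleaning capacity on a widget component.
; The InteractableCleaningCupboard component holds the current phase, which is pushed to WB_CleaningStation_Widget through SetPhase.
; The display refreshes on BeginPlay and on the component's interaction and health-regeneration events, with the widget's shadow casting disabled at start.
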(event `self.ReceiveBeginPlay`
  ;[0.3096 0.5448 0 0.5] BeginPlay
  (bind _aswb_cleaning_station_widget (cast `/Game/Blueprints/Actor/Interaction/Interactable/WB_CleaningStation_Widget` (`WidgetComponent.GetWidget` (`self.CurrentCleaningCapacity`))))
  (`/Game/Blueprints/Actor/Interaction/Interactable/WB_CleaningStation_Widget.SetPhase` _aswb_cleaning_station_widget (`InteractableCleaningCupboard.m_iCurrentPhase` (`self.InteractableCleaningCupboard`)))
  (`PrimitiveComponent.SetCastShadow` (`self.CurrentCleaningCapacity`) false))

(event `self.InteractableCleaningCupboard.OnInteraction`
  ;[0.7698 0.4613 0 0.5] On Interaction Event
  (bind _aswb_cleaning_station_widget (cast `/Game/Blueprints/Actor/Interaction/Interactable/WB_CleaningStation_Widget` (`WidgetComponent.GetWidget` (`self.CurrentCleaningCapacity`))))
  (`/Game/Blueprints/Actor/Interaction/Interactable/WB_CleaningStation_Widget.SetPhase` _aswb_cleaning_station_widget (`InteractableCleaningCupboard.m_iCurrentPhase` (`self.InteractableCleaningCupboard`))))

(event `self.InteractableCleaningCupboard.OnRegenerateHealth`
  (params (health :type Integer))
  ;[0.6352 0.6406 0 0.5] On Regenerate Health Event
  (bind _aswb_cleaning_station_widget (cast `/Game/Blueprints/Actor/Interaction/Interactable/WB_CleaningStation_Widget` (`WidgetComponent.GetWidget` (`self.CurrentCleaningCapacity`))))
  (`/Game/Blueprints/Actor/Interaction/Interactable/WB_CleaningStation_Widget.SetPhase` _aswb_cleaning_station_widget (`InteractableCleaningCupboard.m_iCurrentPhase` (`self.InteractableCleaningCupboard`))))

(fn `UserConstructionScript`)