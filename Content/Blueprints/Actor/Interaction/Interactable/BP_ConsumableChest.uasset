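; BP_ConsumableChest is an interactable consumable chest that animates its door and drawers opening and closing.
; BeginPlay sets separate play rates for three timelines that lerp the door's relative rotation and slide two drawers (Cajao3, Cajao1) along local Y.
; openDrawerAnimation plays them forward with staggered delays, and closeDrawerAnimation reverses the same timelines with its own delays.
; The file contains only this animation, with no item or consumable logic.
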(event `self.ReceiveBeginPlay`
  ;[1 0.2719 0 0.5] begin play
  (`|ExecutionSequence`
    (:`then_0`
      ;;[1 0.2719 0 0.5] set timelines speed
      (`|ExecutionSequence`
        (:`then_0`
          (`TimelineComponent.SetPlayRate` (`self.door`) 1.2))
        (:`then_1`
          (`TimelineComponent.SetPlayRate` (`self.bigCajao`) 1.5))
        (:`then_2`
          (`TimelineComponent.SetPlayRate` (`self.smallLeftCajao`) 1.0))))))

(event `openDrawerAnimation`
  (bind _cajao_1 (`self.cajao_1`))
  (bind _cajao_3 (`self.cajao_3`))
  (bind (_relativelocation_x _relativelocation_y _relativelocation_z) (`KismetMathLibrary.BreakVector` (`SceneComponent.RelativeLocation` _cajao_1)))
  (bind (_relativelocation_x_2 _relativelocation_y_2 _relativelocation_z_2) (`KismetMathLibrary.BreakVector` (`SceneComponent.RelativeLocation` _cajao_3)))
  (`|ExecutionSequence`
    (:`then_0`
      (`KismetSystemLibrary.Delay` 0.4)
      ;[0.06448 0 1 0.5] dooringPuerta
      (bind (_direction _pista_nueva_0) (`Timeline|door` :!via `PlayFromStart` :!label _label)
        (:`Update`
          (bind (_returnvalue_x _returnvalue_y _returnvalue_z) (`KismetMathLibrary.BreakVector` (`KismetMathLibrary.VLerp` (0.0 0.0 0.0) (7.58 1.34 -35.0) _pista_nueva_0)))
          (`SceneComponent.K2_SetRelativeRotation` (`self.dooringPuerta`) (`KismetMathLibrary.MakeRotator` _returnvalue_x _returnvalue_y _returnvalue_z) false false))))
    (:`then_1`
      (`KismetSystemLibrary.Delay` 0.2)
      ;[0 0.3839 1 0.5] big cajao
      (bind (_direction_2 _pista_nueva_0_2) (`Timeline|bigCajao` :!via `PlayFromStart` :!label _label_2)
        (:`Update`
          (`SceneComponent.K2_SetRelativeLocation` _cajao_3 (`KismetMathLibrary.MakeVector` _relativelocation_x_2 (`KismetMathLibrary.Lerp` -37.0 -9.0 _pista_nueva_0_2) _relativelocation_z_2) false false))))
    (:`then_2`
      (`KismetSystemLibrary.Delay` 0.3)
      ;[0 0.3839 1 0.5] small left cajao
      (bind (_direction_3 _pista_nueva_0_3) (`Timeline|smallLeftCajao` :!via `PlayFromStart` :!label _label_3)
        (:`Update`
          (`SceneComponent.K2_SetRelativeLocation` _cajao_1 (`KismetMathLibrary.MakeVector` _relativelocation_x (`KismetMathLibrary.Lerp` -23.0 -8.0 _pista_nueva_0_3) _relativelocation_z) false false))))))

(event `closeDrawerAnimation`
  (`|ExecutionSequence`
    (:`then_0`
      (`KismetSystemLibrary.Delay` 0.0)
      (goto _label :!via `ReverseFromEnd`))
    (:`then_1`
      (`KismetSystemLibrary.Delay` 0.5)
      (goto _label_2 :!via `ReverseFromEnd`))
    (:`then_2`
      (`KismetSystemLibrary.Delay` 0.2)
      (goto _label_3 :!via `ReverseFromEnd`))))

(fn `UserConstructionScript`)