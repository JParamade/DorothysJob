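; BP_DustPoop is a dust poop actor that flashes red whenever its health changes.
; On BeginPlay it binds to a health-changed event, which clears the mesh overlay and swaps the base material to red.
; A half-second timer then restores the dirt material and poop overlay.
; Each new health change cancels any pending timer, so repeated changes extend the flash.
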(event `self.ReceiveBeginPlay`
  (add `self.OnHealthChanged` (delegate `OnHealthChangedEvent`)))

(event `OnHealthChangedEvent`
  (bind _m_pmeshcomponent (`self.m_pMeshComponent`))
  (if (`KismetSystemLibrary.K2_IsValidTimerHandle` (`self.TimerHandle`))
    (`KismetSystemLibrary.K2_ClearAndInvalidateTimerHandle` (`self.TimerHandle`)))
  (`MeshComponent.SetOverlayMaterial` _m_pmeshcomponent null)
  (`PrimitiveComponent.SetMaterial` _m_pmeshcomponent 0 "/Game/Blueprints/Actor/Interaction/Interactable/MI_Red.MI_Red")
  (bind _returnvalue (`KismetSystemLibrary.K2_SetTimerDelegate` (delegate `SetBaseMaterial`) 0.5))
  (set `self.TimerHandle` _returnvalue))

(event `SetBaseMaterial`
  (bind _m_pmeshcomponent (`self.m_pMeshComponent`))
  (`MeshComponent.SetOverlayMaterial` _m_pmeshcomponent "/Game/Graphics/VFX/Material/M_Dust_poop.M_Dust_poop")
  (`PrimitiveComponent.SetMaterial` _m_pmeshcomponent 0 "/Game/Graphics/VFX/Dirt/M_DustDirt.M_DustDirt"))

(fn `UserConstructionScript`)